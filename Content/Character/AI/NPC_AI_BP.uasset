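; NPC AI controller that runs the PatrollingGuard behavior tree and tracks the player through AI perception.
; On BeginPlay it sets up the PatrolData blackboard, starts the tree and caches the blackboard component.
; Perception updates store a sensed actor tagged Player in the Enemy key.
; When that actor stops being sensed, the key and the controller's focus are cleared.
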(event `self.ReceiveBeginPlay`
  (bind _blackboardcomponent (`self.UseBlackboard` "/Game/Character/AI/PatrolData.PatrolData"))
  (`self.RunBehaviorTree` "/Game/Character/AI/PatrollingGuard.PatrollingGuard")
  (set `self.BlackboardComp` _blackboardcomponent))

(event `self.AIPerception.OnTargetPerceptionUpdated`
  (params (Actor :type "Actor Object Reference") (Stimulus :type "AIStimulus Structure"))
  (bind _enemy (`self.Enemy`))
  (bind _blackboardcomp (`self.BlackboardComp`))
  (if (`KismetSystemLibrary.IsValid` Actor)
    (if (`self.ActorHasTag` Actor "Player")
      (if (`.bSuccessfullySensed` (break `AIStimulus` Stimulus))
        (`BlackboardComponent.SetValueAsObject` _blackboardcomp _enemy Actor)
        (else
          (`BlackboardComponent.ClearValue` _blackboardcomp _enemy)
          (`self.K2_ClearFocus`))))))

(fn `UserConstructionScript`)