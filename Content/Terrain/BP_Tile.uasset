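; BP_Tile is an infinite-terrain tile that scatters props and rocks on BeginPlay via PlaceActor and starts with its gate locked.
; When the player enters LockingVolume, the gate opens and turns green, and BP_InfinateTerrain is told to spawn and count the tile conquered.
; Leaving that volume relocks the gate in red, while leaving DestoryVolume destroys the tile.
; GetAttachLocation exposes the Arrow's world transform as an attach point.
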(event `self.ReceiveBeginPlay`
  (`self.Lock`)
  (`self.PlaceActor` "/Game/Terrain/Props/BP_Container.BP_Container_C" 1 5 400.0)
  (`self.PlaceActor` "/Game/Terrain/Props/BP_Canister1.BP_Canister1_C" 1 4 50.0)
  (`self.PlaceActor` "/Game/Terrain/Props/BP_Sack1.BP_Sack1_C" 1 4 150.0)
  (`self.PlaceActor` "/Game/Terrain/Props/BP_Box.BP_Box_C" 1 5 300.0)
  (`self.PlaceActor` "/Game/Terrain/Props/BP_Rock01.BP_Rock01_C" 1 4 264.0 1.0 5.0)
  (`self.PlaceActor` "/Game/Terrain/Props/BP_Rock05.BP_Rock05_C" 1 4 395.0 1.0 5.0)
  (`self.PlaceActor` "/Game/Terrain/Props/BP_Rock17.BP_Rock17_C" 1 5 423.0 1.0 5.0))

(event `self.Locking Volume.OnComponentBeginOverlap`
  (params (OverlappedComponent :type "PrimitiveComponent Object Reference") (OtherActor :type "Actor Object Reference") (OtherComp :type "PrimitiveComponent Object Reference") (OtherBodyIndex :type Integer) (bFromSweep :type Boolean) (SweepResult :type "HitResult Structure (by ref)"))
  (`self.IsPlayer` OtherActor)
  (`self.Unlock`)
  (`PrimitiveComponent.SetMaterial` (`self.Gate`) 0 "/Game/Terrain/MI_Barrier_Green.MI_Barrier_Green")
  (bind _asbp_infinate_terrain (cast `/Game/Levels/BP_InfinateTerrain` (`GameplayStatics.GetGameMode`)))
  (`/Game/Levels/BP_InfinateTerrain.Spawn` _asbp_infinate_terrain)
  (`/Game/Levels/BP_InfinateTerrain.Tile Conquered` _asbp_infinate_terrain))

(event `self.Locking Volume.OnComponentEndOverlap`
  (params (OverlappedComponent :type "PrimitiveComponent Object Reference") (OtherActor :type "Actor Object Reference") (OtherComp :type "PrimitiveComponent Object Reference") (OtherBodyIndex :type Integer))
  (`self.IsPlayer` OtherActor)
  (`self.Lock`)
  (`PrimitiveComponent.SetMaterial` (`self.Gate`) 0 "/Game/Terrain/MI_Barrier_Red.MI_Barrier_Red"))

(event `self.Destory Volume.OnComponentEndOverlap`
  (params (OverlappedComponent :type "PrimitiveComponent Object Reference") (OtherActor :type "Actor Object Reference") (OtherComp :type "PrimitiveComponent Object Reference") (OtherBodyIndex :type Integer))
  (`self.IsPlayer` OtherActor)
  (`self.K2_DestroyActor`))

(fn `Get Attach Location`
  (returns (AttachLocation :type "Transform Structure"))
  (return (`SceneComponent.K2_GetComponentToWorld` (`self.Arrow`))))

(fn `Lock`
  (`PrimitiveComponent.SetCollisionEnabled` (`self.Gate`) "QueryAndPhysics"))

(fn `Unlock`
  (`PrimitiveComponent.SetCollisionEnabled` (`self.Gate`) "NoCollision"))

(fn `UserConstructionScript`)