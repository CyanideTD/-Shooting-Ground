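; Manages endless terrain by spawning BP_Tile actors end to end and keeping a score of conquered tiles.
; BeginPlay populates a nav mesh bounds volume pool, which is handed to each new tile.
; Spawn places a tile, has it populate BP_Character AI pawns in numbers scaled by difficulty, then takes its attach location as the next spawn point.
; TileConquered increments the score, exposed through GetScore.
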(event `self.ReceiveBeginPlay`
  (`self.PopulateBoundVolumePool`))

(fn `GetScore`
  (returns (Score :type Integer))
  (return (`self.Score`)))

(fn `Spawn`
  (for _ (range 1)
    (bind _returnvalue (`|SpawnActorFromClass` "/Game/Terrain/BP_Tile.BP_Tile_C" (`self.SpawnLocation`) "Undefined" "OverrideRootScale" null null))
    (bind _returnvalue_2 (`self.GetDifficulty`))
    (`KismetSystemLibrary.PrintString` (`KismetStringLibrary.Conv_IntToString` _returnvalue_2))
    (switch `int` _returnvalue_2
      (:`Default`
        (`Tile.PlaceAIPawn` _returnvalue "/Game/Character/Character/BP_Character.BP_Character_C" 1 2 :!label _label))
      (:`0`
        (goto _label))
      (:`1`
        (`Tile.PlaceAIPawn` _returnvalue "/Game/Character/Character/BP_Character.BP_Character_C" 1 4))
      (:`2`
        (`Tile.PlaceAIPawn` _returnvalue "/Game/Character/Character/BP_Character.BP_Character_C" 1 8)))
    (`Tile.SetPool` _returnvalue (`self.NavMeshBoundVolumePool`))
    (bind _attachlocation (`/Game/Terrain/BP_Tile.Get Attach Location` _returnvalue))
    (set `self.SpawnLocation` _attachlocation)))

(fn `Tile Conquered`
  (`/Engine/EditorBlueprintResources/StandardMacros.IncrementInt` (`self.Score`)))

(fn `UserConstructionScript`)